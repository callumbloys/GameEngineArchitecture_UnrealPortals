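; Second portal of a Portal-style linked pair, teleporting overlapping actors to Portal 1's location stored on FirstPersonCharacter.
; For players, it also remaps control yaw and relaunches velocity along Portal 1's forward axis, using hardcoded axis-aligned cases.
; Tick publishes its location, switches the plane to a render-target material once Portal 1 exists, and rotates Portal2View with the player camera.
; New placements briefly move the trigger away and back to refresh overlaps.
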(event OnComponentBeginOverlap(TeleportOnOverlap)
  (params (OverlappedComponent :type Primitive%20Component%20Object%20Reference) (OtherActor :type Actor%20Object%20Reference) (OtherComp :type Primitive%20Component%20Object%20Reference) (OtherBodyIndex :type Integer) (bFromSweep :type Boolean) (SweepResult :type Hit%20Result%20Structure%20%28by%20ref%29))
  (if (Variables|Default|GetIsSecondPortalMade)
    (Utilities|Casting|CastToFirstPersonCharacter OtherActor
      (:then
        (Variables|Default|SetIsPlayer true))
      (:CastFailed
        (Variables|Default|SetIsPlayer false)))
    (Variables|Default|SetPortal2ForwardVector (Variables|/Game/FirstPersonBP/Blueprints/FirstPersonCharacter.FirstPersonCharacter_C|GetPortal2ForwardVector (Variables|Default|GetCast%20To%20FPC)))
    (if (Variables|/Game/FirstPersonBP/Blueprints/FirstPersonCharacter.FirstPersonCharacter_C|GetCanTeleport (Variables|Default|GetCast%20To%20FPC))
      (Variables|/Game/FirstPersonBP/Blueprints/FirstPersonCharacter.FirstPersonCharacter_C|SetCanTeleport (Variables|Default|GetCast%20To%20FPC) false)
      (Transformation|SetActorLocation OtherActor (Variables|/Game/FirstPersonBP/Blueprints/FirstPersonCharacter.FirstPersonCharacter_C|GetPortal1 (Variables|Default|GetCast%20To%20FPC)) false true)
      (Transformation|SetActorScale3D OtherActor "0.300000,0.300000,0.300000")
      (if (Variables|Default|GetIsPlayer)
        (CallFunction|SetPlayerRotation)
        (CallFunction|SetPlayerVelocity))
      (Default|ResetCanTeleport (Variables|Default|GetCast%20To%20FPC)))))

(event Custom|ChangeOverlapPosition
  (Variables|Default|SetCollisionOriginalLocation (Transformation|GetWorldLocation (Variables|Default|GetTeleportOnOverlap)))
  (Transformation|SetWorldLocation (Variables|Default|GetTeleportOnOverlap) (Variables|Default|GetCollisionRandomLocation) false true)
  (Utilities|FlowControl|Delay 0.1)
  (Transformation|SetWorldLocation (Variables|Default|GetTeleportOnOverlap) (Variables|Default|GetCollisionOriginalLocation) false true)
  (if (Variables|Default|GetFirstRun)
    (Variables|Default|SetFirstRun false)
    (else
      (Variables|/Game/FirstPersonBP/Blueprints/FirstPersonCharacter.FirstPersonCharacter_C|SetNewlyCreatedPortal2 (Variables|Default|GetCast%20To%20FPC) false))))

(event EventBeginPlay
  (bind _asfirst_person_character (Utilities|Casting|CastToFirstPersonCharacter (Game|GetPlayerCharacter 0)))
  (Variables|Default|SetCast%20To%20FPC _asfirst_person_character)
  (Variables|Default|SetCollisionOriginalLocation (Transformation|GetWorldLocation (Variables|Default|GetTeleportOnOverlap)))
  (Transformation|SetWorldLocation (Variables|Default|GetTeleportOnOverlap) (Variables|Default|GetCollisionRandomLocation) false true)
  (Utilities|FlowControl|Delay 0.1)
  (Transformation|SetWorldLocation (Variables|Default|GetTeleportOnOverlap) (Variables|Default|GetCollisionOriginalLocation) false true)
  (if (Variables|Default|GetFirstRun)
    (Variables|Default|SetFirstRun false)
    (else
      (Variables|/Game/FirstPersonBP/Blueprints/FirstPersonCharacter.FirstPersonCharacter_C|SetNewlyCreatedPortal2 (Variables|Default|GetCast%20To%20FPC) false))))

(event Collision|EventActorBeginOverlap
  (params (OtherActor :type Actor%20Object%20Reference)))

(event EventTick
  (params (DeltaSeconds :type Float%20%28single-precision%29))
  (Variables|/Game/FirstPersonBP/Blueprints/FirstPersonCharacter.FirstPersonCharacter_C|SetPortal2 (Variables|Default|GetCast%20To%20FPC) (Transformation|GetWorldLocation (Variables|Default|GetDefaultSceneRoot)))
  (if (Math|Vector|Equal(Vector) (Variables|/Game/FirstPersonBP/Blueprints/FirstPersonCharacter.FirstPersonCharacter_C|GetPortal1 (Variables|Default|GetCast%20To%20FPC)) "0, 0, 0" 1.0)
    (Rendering|Material|SetMaterial (Variables|Default|GetPlane) 0 "/Game/Blueprint/NoPortal1Created.NoPortal1Created")
    (else
      (Rendering|Material|SetMaterial (Variables|Default|GetPlane) 0 "/Game/Blueprint/Portal2_RT_Mat.Portal2_RT_Mat")
      (Variables|Default|SetIsSecondPortalMade true)
      (if (Variables|/Game/FirstPersonBP/Blueprints/FirstPersonCharacter.FirstPersonCharacter_C|GetNewlyCreatedPortal2 (Variables|Default|GetCast%20To%20FPC))
        (CallFunction|ChangeOverlapPosition))
      (CallFunction|SetRenderTargetRotation))))

(fn ConstructionScript)

(fn SetPlayerVelocity
  (Variables|/Script/Engine.CharacterMovementComponent|SetMaxAcceleration (Variables|/Script/Engine.Character|GetCharacterMovement (Variables|Default|GetCast%20To%20FPC)) 4096.0)
  (Default|StoreVelocity (Variables|Default|GetCast%20To%20FPC))
  (Variables|Default|SetPortal1ForwardVector (Variables|Default|GetPortal1ForwardVector))
  (CallFunction|SetVelocityAccordingtoForwardVector))

(fn SetPlayerRotation
  (Variables|Default|SetPortal1Rotation (Variables|/Game/FirstPersonBP/Blueprints/FirstPersonCharacter.FirstPersonCharacter_C|GetPortal1Rotation (Variables|Default|GetCast%20To%20FPC)))
  (Variables|Default|SetPortal2Rotation (Transformation|GetWorldRotation (Variables|Default|GetDefaultSceneRoot)))
  (Variables|Default|SetPlayerRotation (Transformation|GetActorRotation (Game|GetPlayerController 0)))
  (Variables|Default|SetPlayerController (Game|GetPlayerController 0))
  ;[1 1 1] If portal 1 Rotation = Portal 2 roatation
  (if (Math|Rotator|Equal(Rotator) (Variables|Default|GetPortal1Rotation) (Variables|Default|GetPortal2Rotation) 1.0)
    (Pawn|SetControlRotation (Variables|Default|GetPlayerController) (Math|Rotator|MakeRotator (.roll (Variables|Default|GetPlayerRotation)) (.pitch (Variables|Default|GetPlayerRotation)) (+ (.yaw (Variables|Default|GetPlayerRotation)) 1.8e+02)))
    (else
      ;[1 1 1] If Portal 1 is opposite axis to portal 2
      (if (Math|Boolean|ORBoolean (Math|Rotator|Equal(Rotator) (* (Variables|Default|GetPortal1Rotation) -1) (Variables|Default|GetPortal2Rotation) 1.0) (and (Math|Rotator|Equal(Rotator) (Variables|Default|GetPortal1Rotation) "0, 0, 0" 1.0) (Math|Rotator|Equal(Rotator) (Variables|Default|GetPortal2Rotation) "0,180.000000, 0" 1.0)) (and (Math|Rotator|Equal(Rotator) (Variables|Default|GetPortal1Rotation) "0,180.000000, 0" 1.0) (Math|Rotator|Equal(Rotator) (Variables|Default|GetPortal2Rotation) "0, 0, 0" 1.0)))
        (Pawn|SetControlRotation (Variables|Default|GetPlayerController) (Math|Rotator|MakeRotator (.roll (Variables|Default|GetPlayerRotation)) (.pitch (Variables|Default|GetPlayerRotation)) (.yaw (Variables|Default|GetPlayerRotation))))
        (else
          ;[1 1 1] If portal 1 has spawned at -X axis
          (if (Math|Rotator|Equal(Rotator) (Variables|Default|GetPortal2Rotation) "0, 0, 0" 1.0)
            (if (Math|Rotator|Equal(Rotator) (Variables|Default|GetPortal1Rotation) "0,90.000000, 0" 1.0)
              (Pawn|SetControlRotation (Variables|Default|GetPlayerController) (Math|Rotator|MakeRotator (.roll (Variables|Default|GetPlayerRotation)) (.pitch (Variables|Default|GetPlayerRotation)) (+ (.yaw (Variables|Default|GetPlayerRotation)) -9e+01)))
              (else
                (Pawn|SetControlRotation (Variables|Default|GetPlayerController) (Math|Rotator|MakeRotator (.roll (Variables|Default|GetPlayerRotation)) (.pitch (Variables|Default|GetPlayerRotation)) (+ (.yaw (Variables|Default|GetPlayerRotation)) 9e+01)))))
            (else
              ;[1 1 1] If portal 1 has spawned at X axis
              (if (Math|Rotator|Equal(Rotator) (Variables|Default|GetPortal2Rotation) "0,180.000000, 0" 1.0)
                (if (Math|Rotator|Equal(Rotator) (Variables|Default|GetPortal1Rotation) "0,90.000000, 0" 1.0)
                  (Pawn|SetControlRotation (Variables|Default|GetPlayerController) (Math|Rotator|MakeRotator (.roll (Variables|Default|GetPlayerRotation)) (.pitch (Variables|Default|GetPlayerRotation)) (+ (.yaw (Variables|Default|GetPlayerRotation)) 9e+01)))
                  (else
                    (Pawn|SetControlRotation (Variables|Default|GetPlayerController) (Math|Rotator|MakeRotator (.roll (Variables|Default|GetPlayerRotation)) (.pitch (Variables|Default|GetPlayerRotation)) (+ (.yaw (Variables|Default|GetPlayerRotation)) -9e+01)))))
                (else
                  ;[1 1 1] If portal 1 has spawned at Y axis
                  (if (Math|Rotator|Equal(Rotator) (Variables|Default|GetPortal2Rotation) "0,-90.000000, 0" 1.0)
                    (if (Math|Rotator|Equal(Rotator) (Variables|Default|GetPortal1Rotation) "0, 0, 0" 1.0)
                      (Pawn|SetControlRotation (Variables|Default|GetPlayerController) (Math|Rotator|MakeRotator (.roll (Variables|Default|GetPlayerRotation)) (.pitch (Variables|Default|GetPlayerRotation)) (+ (.yaw (Variables|Default|GetPlayerRotation)) -9e+01)))
                      (else
                        (Pawn|SetControlRotation (Variables|Default|GetPlayerController) (Math|Rotator|MakeRotator (.roll (Variables|Default|GetPlayerRotation)) (.pitch (Variables|Default|GetPlayerRotation)) (+ (.yaw (Variables|Default|GetPlayerRotation)) 9e+01)))))
                    (else
                      ;[1 1 1] If portal 1 has spawned at -Y axis
                      (if (Math|Rotator|Equal(Rotator) (Variables|Default|GetPortal2Rotation) "0,90.000000, 0" 1.0)
                        (if (Math|Rotator|Equal(Rotator) (Variables|Default|GetPortal1Rotation) "0, 0, 0" 1.0)
                          (Pawn|SetControlRotation (Variables|Default|GetPlayerController) (Math|Rotator|MakeRotator (.roll (Variables|Default|GetPlayerRotation)) (.pitch (Variables|Default|GetPlayerRotation)) (+ (.yaw (Variables|Default|GetPlayerRotation)) 9e+01)))
                          (else
                            (Pawn|SetControlRotation (Variables|Default|GetPlayerController) (Math|Rotator|MakeRotator (.roll (Variables|Default|GetPlayerRotation)) (.pitch (Variables|Default|GetPlayerRotation)) (+ (.yaw (Variables|Default|GetPlayerRotation)) -9e+01)))))
                        (else
                          ;[1 1 1] If portal 1 has spawned at -Y axis
                          (if (Math|Rotator|Equal(Rotator) (Variables|Default|GetPortal2Rotation) "90.000000,0.000000, 0" 1.0)
                            (Pawn|SetControlRotation (Variables|Default|GetPlayerController) (Math|Rotator|MakeRotator (.roll (Variables|Default|GetPlayerRotation)) (.pitch (Variables|Default|GetPlayerRotation)) (.yaw (Variables|Default|GetPortal2Rotation))))))))))))))))))

(fn ResetMaxAcceleration)

(fn SetVelocityAccordingtoForwardVector
  (bind _portal2forwardvector (Variables|Default|GetPortal2ForwardVector))
  (bind _portal1forwardvector (Variables|Default|GetPortal1ForwardVector))
  (bind _portal1forwardvector_2 (Variables|Default|GetPortal1ForwardVector))
  (bind _portal2forwardvector_2 (Variables|Default|GetPortal2ForwardVector))
  (bind _portal1forwardvector_3 (Variables|Default|GetPortal1ForwardVector))
  (bind _portal1forwardvector_4 (Variables|Default|GetPortal1ForwardVector))
  (bind _portal1forwardvector_5 (Variables|Default|GetPortal1ForwardVector))
  (bind _cast_to_fpc (Variables|Default|GetCast%20To%20FPC))
  (bind _portal2forwardvector_3 (Variables|Default|GetPortal2ForwardVector))
  (bind _portal1forwardvector_6 (Variables|Default|GetPortal1ForwardVector))
  (bind _portal1forwardvector_7 (Variables|Default|GetPortal1ForwardVector))
  (bind _portal1forwardvector_8 (Variables|Default|GetPortal1ForwardVector))
  (bind _portal1forwardvector_9 (Variables|Default|GetPortal1ForwardVector))
  (bind _playervelocity (Variables|/Game/FirstPersonBP/Blueprints/FirstPersonCharacter.FirstPersonCharacter_C|GetPlayerVelocity _cast_to_fpc))
  (bind _returnvalue (Math|Float|Absolute(Float) (.z _playervelocity)))
  ;[1 1 1] If forward vector of portal 1 is X then set player velocity to forward vector of portal 2
  (if (or (== (.x _portal2forwardvector_2) 1.0) (== (.x _portal2forwardvector_2) -1.0))
    (if (or (== (.x _portal1forwardvector_3) 1.0) (== (.x _portal1forwardvector_3) -1.0))
      (Character|LaunchCharacter (Variables|Default|GetCast%20To%20FPC) (Math|Vector|MakeVector (* (+ (Math|Float|Absolute(Float) (.x (Variables|/Game/FirstPersonBP/Blueprints/FirstPersonCharacter.FirstPersonCharacter_C|GetPlayerVelocity (Variables|Default|GetCast%20To%20FPC)))) (Variables|Default|GetVelocityAddition)) (.x _portal1forwardvector_3)) 0.0 0.0) true true)
      (elif (or (== (.y _portal1forwardvector_4) 1.0) (== (.y _portal1forwardvector_4) -1.0))
        (Character|LaunchCharacter (Variables|Default|GetCast%20To%20FPC) (Math|Vector|MakeVector 0.0 (* (+ (Math|Float|Absolute(Float) (.x (Variables|/Game/FirstPersonBP/Blueprints/FirstPersonCharacter.FirstPersonCharacter_C|GetPlayerVelocity (Variables|Default|GetCast%20To%20FPC)))) (Variables|Default|GetVelocityAddition)) (.y _portal1forwardvector_4)) 0.0) true true)
        (elif (or (== (.z _portal1forwardvector_5) 1.0) (== (.z _portal1forwardvector_5) -1.0))
          (Character|LaunchCharacter (Variables|Default|GetCast%20To%20FPC) (Math|Vector|MakeVector 0.0 0.0 (* (+ (Math|Float|Absolute(Float) (.x (Variables|/Game/FirstPersonBP/Blueprints/FirstPersonCharacter.FirstPersonCharacter_C|GetPlayerVelocity (Variables|Default|GetCast%20To%20FPC)))) (Variables|Default|GetVelocityAdditionZVector)) (.z _portal1forwardvector_5))) true true))))
    (else
      ;[1 1 1] If forward vector of portal 1 is Y then set player velocity to forward vector of portal 2
      (if (or (== (.y _portal2forwardvector_3) 1.0) (== (.y _portal2forwardvector_3) -1.0))
        (if (or (== (.x _portal1forwardvector_6) 1.0) (== (.x _portal1forwardvector_6) -1.0))
          (Character|LaunchCharacter (Variables|Default|GetCast%20To%20FPC) (Math|Vector|MakeVector (* (+ (Math|Float|Absolute(Float) (.y (Variables|/Game/FirstPersonBP/Blueprints/FirstPersonCharacter.FirstPersonCharacter_C|GetPlayerVelocity (Variables|Default|GetCast%20To%20FPC)))) (Variables|Default|GetVelocityAddition)) (.x _portal1forwardvector_6)) 0.0 0.0) true true)
          (elif (or (== (.y _portal1forwardvector_7) 1.0) (== (.y _portal1forwardvector_7) -1.0))
            (Character|LaunchCharacter (Variables|Default|GetCast%20To%20FPC) (Math|Vector|MakeVector 0.0 (* (+ (Math|Float|Absolute(Float) (.y (Variables|/Game/FirstPersonBP/Blueprints/FirstPersonCharacter.FirstPersonCharacter_C|GetPlayerVelocity (Variables|Default|GetCast%20To%20FPC)))) (Variables|Default|GetVelocityAddition)) (.y _portal1forwardvector_7)) 0.0) true true)
            (elif (or (== (.z _portal1forwardvector_8) 1.0) (== (.z _portal1forwardvector_8) -1.0))
              (Character|LaunchCharacter (Variables|Default|GetCast%20To%20FPC) (Math|Vector|MakeVector 0.0 0.0 (* (+ (Math|Float|Absolute(Float) (.y (Variables|/Game/FirstPersonBP/Blueprints/FirstPersonCharacter.FirstPersonCharacter_C|GetPlayerVelocity (Variables|Default|GetCast%20To%20FPC)))) (Variables|Default|GetVelocityAdditionZVector)) (.z _portal1forwardvector_8))) true true))))
        (else
          ;[1 1 1] If forward vector of portal 1 is Y then set player velocity to forward vector of portal 2
          (if (or (== (.z _portal2forwardvector) 1.0) (== (.z _portal2forwardvector) -1.0))
            (if (or (== (.x _portal1forwardvector_9) 1.0) (== (.x _portal1forwardvector_9) -1.0))
              (Character|LaunchCharacter (Variables|Default|GetCast%20To%20FPC) (Math|Vector|MakeVector (* (+ (Math|Float|Absolute(Float) (.z (Variables|/Game/FirstPersonBP/Blueprints/FirstPersonCharacter.FirstPersonCharacter_C|GetPlayerVelocity (Variables|Default|GetCast%20To%20FPC)))) (Variables|Default|GetVelocityAdditionZVector)) (.x _portal1forwardvector_9)) 0.0 0.0) true true)
              (elif (or (== (.y _portal1forwardvector_2) 1.0) (== (.y _portal1forwardvector_2) -1.0))
                (Character|LaunchCharacter (Variables|Default|GetCast%20To%20FPC) (Math|Vector|MakeVector 0.0 (* (+ (Math|Float|Absolute(Float) (.z (Variables|/Game/FirstPersonBP/Blueprints/FirstPersonCharacter.FirstPersonCharacter_C|GetPlayerVelocity (Variables|Default|GetCast%20To%20FPC)))) (Variables|Default|GetVelocityAddition)) (.y _portal1forwardvector_2)) 0.0) true true)
                (elif (or (== (.z _portal1forwardvector) 1.0) (== (.z _portal1forwardvector) -1.0))
                  (if (<= _returnvalue 5e+02)
                    (Variables|Default|SetSetIndex 0)
                    (else
                      (Variables|Default|SetSetIndex 1)))
                  (Character|LaunchCharacter (Variables|Default|GetCast%20To%20FPC) (Math|Vector|MakeVector 0.0 0.0 (Utilities|Select :Index (Variables|Default|GetSetIndex) :Option%200 (* (Variables|Default|GetVelocityAdditionZVector) (.z _playervelocity)) :Option%201 (* (+ _returnvalue 5e+01) (.z _playervelocity)))) true true))))))))))

(fn SetPortal1LocationonCall)

(fn SetRenderTargetRotation
  (Variables|Default|SetPlayerRotation (Transformation|GetWorldRotation (Variables|/Script/Engine.PlayerCameraManager|GetTransformComponent (Game|GetPlayerCameraManager 0))))
  (Variables|Default|SetPortal1ForwardVector (Variables|/Game/FirstPersonBP/Blueprints/FirstPersonCharacter.FirstPersonCharacter_C|GetPortal1ForwardVector (Variables|Default|GetCast%20To%20FPC)))
  (if (== (.x (Variables|Default|GetPortal1ForwardVector)) 1.0)
    (Transformation|SetRelativeRotation (Variables|Default|GetPortal2View) (Math|Rotator|MakeRotator 0.0 (* 1 (.pitch (Variables|Default|GetPlayerRotation))) (* -1 (- 1.8e+02 (.yaw (Variables|Default|GetPlayerRotation))))) false false)
    (elif (== (.x (Variables|Default|GetPortal1ForwardVector)) -1.0)
      (Transformation|SetRelativeRotation (Variables|Default|GetPortal2View) (Math|Rotator|MakeRotator 0.0 (.pitch (Variables|Default|GetPlayerRotation)) (.yaw (Variables|Default|GetPlayerRotation))) false false)
      (elif (== (.y (Variables|Default|GetPortal1ForwardVector)) 1.0)
        (Transformation|SetRelativeRotation (Variables|Default|GetPortal2View) (Math|Rotator|MakeRotator 0.0 (* 1 (.pitch (Variables|Default|GetPlayerRotation))) (* -1 (- -9e+01 (.yaw (Variables|Default|GetPlayerRotation))))) false false)
        (elif (== (.y (Variables|Default|GetPortal1ForwardVector)) -1.0)
          (Transformation|SetRelativeRotation (Variables|Default|GetPortal2View) (Math|Rotator|MakeRotator 0.0 (.pitch (Variables|Default|GetPlayerRotation)) (* -1 (- 9e+01 (.yaw (Variables|Default|GetPlayerRotation))))) false false))))))